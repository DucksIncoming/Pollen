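; Placeable flower building that follows the player's aim while being placed, then grows through mesh stages over time.
; While placing, a camera trace positions and surface-aligns the mesh, with custom depth and green or red post-process volumes signalling validity.
; Place requires a downward trace hitting WorldStatic, then consumes a hotbar item.
; DefineFlower sets up the mesh, tags and age-threshold map that Grow uses to swap meshes.
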(event EventBeginPlay
  (Variables|Default|SetRandomRotation (Math|Rotator|MakeRotator 0.0 0.0 (* (Math|Trig|Sin(Radians) (* (Utilities|Time|GetGameTimeinSeconds) 1e+03)) 1.8e+02)))
  (bind _asbp_player (Utilities|Casting|CastToBP_Player (Game|GetPlayerCharacter 0)))
  (Variables|Default|SetPlayerRef _asbp_player)
  (bind _outactors (Actor|GetAllActorsOfClass "/Script/Engine.PostProcessVolume"))
  (for _array_element _outactors
    (switch string (Utilities|GetDisplayName _array_element)
      (:PPV_Green
        (Variables|Default|SetPPV_Green _array_element))
      (:PPV_Neutral
        (Variables|Default|SetPPV_Neutral _array_element))
      (:PPV_Red
        (Variables|Default|SetPPV_Red _array_element))))
  (CallFunction|Grow 0.0))

(event EventTick
  (params (DeltaSeconds :type Float%20%28single-precision%29))
  (bind _playerref (Variables|Default|GetPlayerRef))
  (bind _playerref_2 (Variables|Default|GetPlayerRef))
  (bind _camera (Variables|/Game/Assets/Blueprints/Player/BP_Player.BP_Player_C|GetCamera _playerref))
  (bind _camera_2 (Variables|/Game/Assets/Blueprints/Player/BP_Player.BP_Player_C|GetCamera _playerref_2))
  (bind _returnvalue (Transformation|GetWorldLocation _camera_2))
  (if (Variables|Default|GetPlacing)
    (CallFunction|SetColor true)
    (bind _result (CallFunction|CheckValidPlacement))
    (for (_array_element _array_index) (Utilities|Array|MakeArray false (not _result) _result)
      (Variables|/Script/Engine.PostProcessVolume|SetbUnbound (Utilities|Array|Get(acopy) (Utilities|Array|MakeArray (Variables|Default|GetPPV_Neutral) (Variables|Default|GetPPV_Red) (Variables|Default|GetPPV_Green)) _array_index) _array_element)
      (bind (_outhit _returnvalue_2) (Collision|LineTraceForObjects _returnvalue (+ _returnvalue (* (Math|Vector|GetForwardVector _camera_2) 8e+02)) (Utilities|Array|MakeArray "ObjectTypeQuery1" "ObjectTypeQuery9" "ObjectTypeQuery8") false 0 "None"))
      (Transformation|SetWorldLocation (Variables|Default|GetStaticMesh) (Utilities|Array|Get(acopy) (Utilities|Array|MakeArray (+ (Transformation|GetWorldLocation _camera) (* (Math|Vector|GetForwardVector _camera) 8e+02)) (.location _outhit)) (Math|Conversions|ToInteger(Boolean) _returnvalue_2)) false false)
      (Transformation|SetWorldRotation (Variables|Default|GetStaticMesh) (Math|Rotator|CombineRotators (Math|Rotator|CombineRotators (Math|Rotator|CombineRotators (Math|Rotator|MakeRotfromZ (.impactnormal _outhit)) (Variables|Default|GetRotationMemory)) (Math|Rotator|MakeRotator 0.0 0.0 (.yaw (Transformation|GetWorldRotation (Variables|/Game/Assets/Blueprints/Player/BP_Player.BP_Player_C|GetCamera (Variables|Default|GetPlayerRef)))))) (Variables|Default|GetRandomRotation)) false false))
    (else
      (CallFunction|Grow DeltaSeconds)
      (CallFunction|SetColor false))))

(fn ConstructionScript)

(fn DefineFlower
  (params (Name :type String) (Mesh :type Map%20of%20Static%20Mesh%20Object%20References%20to%20Reals) (Transform :type Transform) (HP :type Float%20%28double-precision%29))
  (Variables|Default|SetName Name)
  (bind _output_get (Variables|Default|SetGrowthStages Mesh))
  (bind _keys (Utilities|Map|Keys _output_get))
  (Variables|Default|SetMesh (Utilities|Array|Get(acopy) _keys))
  (Variables|Default|SetHP HP)
  (bind _output_get_2 (Variables|Default|SetTransform Transform))
  (Transformation|SetRelativeScale3D (Variables|Default|GetStaticMesh) (.scale _output_get_2))
  (Variables|Default|SetRotationMemory (.rotation _output_get_2))
  (Collision|SetCollisionObjectType (Variables|Default|GetStaticMesh) "ECC_GameTraceChannel4")
  (Collision|SetCollisionEnabled (Variables|Default|GetStaticMesh) "NoCollision")
  (Components|StaticMesh|SetStaticMesh (Variables|Default|GetStaticMesh) (Variables|Default|GetMesh))
  (Variables|/Script/Engine.ActorComponent|SetComponentTags (Variables|Default|GetStaticMesh) (Utilities|Array|MakeArray "Building" (Utilities|String|StringToName (Variables|Default|GetName)) (Utilities|String|StringToName (Utilities|String|ToString(Float) (Variables|Default|GetHP)))))
  (return (Variables|Default|GetStaticMesh)))

(fn Place
  (bind _playerref (Variables|Default|GetPlayerRef))
  (bind _result (CallFunction|CheckValidPlacement))
  (if _result
    (bind _values (Utilities|Map|Values (Variables|/Game/Assets/Blueprints/Player/BP_Player.BP_Player_C|GetHotbarCount _playerref)))
    (if (> (Utilities|Array|Get(acopy) _values (Variables|/Game/Assets/Blueprints/Player/BP_Player.BP_Player_C|GetHotbarActiveSlot _playerref)) 0)
      (Default|RemoveItem (Variables|Default|GetPlayerRef) (Variables|Default|GetName) 1)
      (Variables|Default|SetPlacing false)
      (Variables|/Game/Assets/Blueprints/Player/BP_Player.BP_Player_C|SetFlowerRotationMemory (Variables|Default|GetPlayerRef) (Variables|Default|GetRotationMemory))
      (Variables|/Game/Assets/Blueprints/Player/BP_Player.BP_Player_C|SetFlowerMemory (Variables|Default|GetPlayerRef) 0))))

(fn CheckValidPlacement
  (bind _staticmesh (Variables|Default|GetStaticMesh))
  (bind (_origin _boxextent) (Collision|GetComponentBounds _staticmesh))
  (bind _outhit (Collision|LineTraceForObjects (+ _origin (Math|Vector|MakeVector 0.0 0.0 (.z _boxextent))) (- _origin (Math|Vector|MakeVector 0.0 0.0 (.z _boxextent))) (Utilities|Array|MakeArray "ObjectTypeQuery8" "ObjectTypeQuery9" "ObjectTypeQuery1") false 0 "None" true "(R=1.000000,G=0.000000,B=0.000000,A=1.000000)" "(R=0.000000,G=1.000000,B=0.000000,A=1.000000)" 0.1))
  (Utilities|IsValid (.hitcomponent _outhit)
    (:Is%20Valid
      (return (Utilities|Enum|Equal(Enum) (Collision|GetCollisionObjectType (.hitcomponent _outhit)) "ECC_WorldStatic")))
    (:Is%20Not%20Valid
      (return false))))

(fn SetColor
  (params (Highlight :type Boolean))
  (bind _staticmesh (Variables|Default|GetStaticMesh))
  (if Highlight
    (Rendering|SetRenderCustomDepth _staticmesh true)
    (else
      (Rendering|SetRenderCustomDepth _staticmesh false))))

(fn Grow
  (params (Delta%20Time :type Float%20%28double-precision%29))
  (Variables|Default|SetAge (+ Delta%20Time (Variables|Default|GetAge)))
  (bind _values (Utilities|Map|Values (Variables|Default|GetGrowthStages)))
  (for (_array_element _array_index) _values
    (bind _keys (Utilities|Map|Keys (Variables|Default|GetGrowthStages)))
    (Components|StaticMesh|SetStaticMesh (Variables|Default|GetStaticMesh) (Utilities|Array|Get(acopy) (Utilities|Array|MakeArray (Variables|Default|GetMesh) (Utilities|Array|Get(acopy) _keys _array_index)) (Math|Conversions|ToInteger(Boolean) (> (Variables|Default|GetAge) _array_element))))
    (Variables|Default|SetMesh (Utilities|Array|Get(acopy) (Utilities|Array|MakeArray (Variables|Default|GetMesh) (Utilities|Array|Get(acopy) _keys _array_index)) (Math|Conversions|ToInteger(Boolean) (> (Variables|Default|GetAge) _array_element))))))