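; BP_Item is a world item actor that destroys itself after a set despawn time and simulates physics only near the player.
; BeginPlay caches the player as BP_Player, then starts the despawn delay.
; Every Tick, it enables or disables mesh physics by comparing the distance between the mesh's relative location and the player's actor location against a simulation distance.
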(event EventBeginPlay
  (bind _asbp_player (Utilities|Casting|CastToBP_Player (Game|GetPlayerCharacter 0))
    (:then
      (Variables|Default|SetPlayerRef _asbp_player))
    (:CastFailed
      _))
  (Utilities|FlowControl|Delay (Variables|Default|GetDespawnTime))
  (Actor|DestroyActor))

(event Collision|EventActorBeginOverlap
  (params (OtherActor :type Actor%20Object%20Reference)))

(event EventTick
  (params (DeltaSeconds :type Float%20%28single-precision%29))
  (bind _mesh (Variables|Default|GetMesh))
  (Utilities|IsValid _mesh
    (:Is%20Valid
      (Physics|SetSimulatePhysics _mesh (< (Math|Vector|Distance(Vector) (Variables|/Script/Engine.SceneComponent|GetRelativeLocation (Variables|Default|GetMesh)) (Transformation|GetActorLocation (Variables|Default|GetPlayerRef))) (Variables|Default|GetSimulationDistance))))))

(fn ConstructionScript)