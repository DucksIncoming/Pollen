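; BP_Buildable is a player-placed building piece, configured through DefineBuilding with name, HP, mesh and other properties.
; While placing, it follows a camera line trace with optional grid snapping, combining 90-degree player yaw with manual rotation.
; A box trace rejects overlaps by piece name, collision type and rotation, toggling red or green post-process volumes over the custom-depth highlight.
; Valid placement consumes the hotbar item, enables collision and saves the rotation on the player.
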(event EventBeginPlay
  (bind _asbp_player (Utilities|Casting|CastToBP_Player (Game|GetPlayerCharacter 0)))
  (Variables|Default|SetPlayerRef _asbp_player)
  (CallFunction|SetColor true)
  (bind _outactors (Actor|GetAllActorsOfClass "/Script/Engine.PostProcessVolume"))
  (for _array_element _outactors
    (switch string (Utilities|GetDisplayName _array_element)
      (:PPV_Green
        (Variables|Default|SetPPV_Green _array_element))
      (:PPV_Neutral
        (Variables|Default|SetPPV_Neutral _array_element))
      (:PPV_Red
        (Variables|Default|SetPPV_Red _array_element)))))

(event EventTick
  (params (DeltaSeconds :type Float%20%28single-precision%29))
  (bind _playerref (Variables|Default|GetPlayerRef))
  (bind _playerref_2 (Variables|Default|GetPlayerRef))
  (bind _camera (Variables|/Game/Assets/Blueprints/Player/BP_Player.BP_Player_C|GetCamera _playerref))
  (bind _camera_2 (Variables|/Game/Assets/Blueprints/Player/BP_Player.BP_Player_C|GetCamera _playerref_2))
  (bind _returnvalue (Transformation|GetWorldLocation _camera_2))
  (if (Variables|Default|GetPlacing)
    (CallFunction|CheckValidPlacement)
    (bind (_outhit _returnvalue_2) (Collision|LineTraceForObjects _returnvalue (+ _returnvalue (* (Math|Vector|GetForwardVector _camera_2) 8e+02)) (Utilities|Array|MakeArray "ObjectTypeQuery1" "ObjectTypeQuery9") false 0 "None"))
    (Variables|Default|SetPlayerRotation (* (Math|Rotator|MakeRotator 0.0 0.0 (Math|Conversions|ToFloat(Integer) (Math|Float|Round (/ (.yaw (Transformation|GetWorldRotation (Variables|/Game/Assets/Blueprints/Player/BP_Player.BP_Player_C|GetCamera (Variables|Default|GetPlayerRef)))) 9e+01)))) 9e+01))
    (Transformation|SetWorldLocation (Variables|Default|GetDefaultSceneRoot) (Utilities|Array|Get(acopy) (Utilities|Array|MakeArray (Utilities|Array|Get(acopy) (Utilities|Array|MakeArray (+ (Transformation|GetWorldLocation _camera) (* (Math|Vector|GetForwardVector _camera) 8e+02)) (.location _outhit)) (Math|Conversions|ToInteger(Boolean) _returnvalue_2)) (Utilities|SnapPostoGrid (Utilities|Array|Get(acopy) (Utilities|Array|MakeArray (+ (Transformation|GetWorldLocation _camera) (* (Math|Vector|GetForwardVector _camera) 8e+02)) (.location _outhit)) (Math|Conversions|ToInteger(Boolean) _returnvalue_2)))) (Math|Conversions|ToInteger(Boolean) (Variables|Default|GetSnapToGrid))) false false)
    (Transformation|SetWorldRotation (Variables|Default|GetDefaultSceneRoot) (Math|Rotator|CombineRotators (Variables|Default|GetManualRotation) (Variables|Default|GetPlayerRotation)) false false)
    (else
      (CallFunction|SetColor false))))

(fn ConstructionScript)

(fn DefineBuilding
  (params (Name :type String) (HP :type Float%20%28double-precision%29) (Material :type String) (Category :type String) (Mesh :type Static%20Mesh%20Object%20Reference) (Transform :type Transform))
  (Variables|Default|SetName Name)
  (Variables|Default|SetHP HP)
  (Variables|Default|SetMaterial Material)
  (Variables|Default|SetCategory Category)
  (Variables|Default|SetMesh Mesh)
  (bind _output_get (Variables|Default|SetTransform Transform))
  (Transformation|SetRelativeScale3D (Variables|Default|GetStaticMesh) (.scale _output_get))
  (Variables|Default|SetManualRotation (.rotation _output_get))
  (Collision|SetCollisionObjectType (Variables|Default|GetStaticMesh) "ECC_GameTraceChannel3")
  (Components|StaticMesh|SetStaticMesh (Variables|Default|GetStaticMesh) Mesh)
  (Variables|/Script/Engine.ActorComponent|SetComponentTags (Variables|Default|GetStaticMesh) (Utilities|Array|MakeArray "Building" (Utilities|String|StringToName Name) (Utilities|String|StringToName (Utilities|String|ToString(Float) HP))))
  (if (Utilities|Enum|Equal(Enum) (Variables|Default|GetName) "Lantern")
    (bind _returnvalue (AddComponent|AddPointLightComponent false (Math|Transform|MakeTransform "40.000000,-190.000000,160.000000" "0, 0, 0" "1.000000,1.000000,1.000000")))
    (return (Variables|Default|GetStaticMesh))
    (else
      (return (Variables|Default|GetStaticMesh)))))

(fn SetColor
  (params (Highlight :type Boolean))
  (bind _asprimitive_component (Utilities|Casting|CastToPrimitiveComponent (Utilities|Array|Get(acopy) (Components|GetChildrenComponents (Variables|Default|GetDefaultSceneRoot) false))))
  (if Highlight
    (Rendering|SetRenderCustomDepth _asprimitive_component true)
    (else
      (Rendering|SetRenderCustomDepth _asprimitive_component false))))

(fn Place
  (bind _playerref (Variables|Default|GetPlayerRef))
  (bind _validplacement (CallFunction|CheckValidPlacement))
  (if _validplacement
    (bind _values (Utilities|Map|Values (Variables|/Game/Assets/Blueprints/Player/BP_Player.BP_Player_C|GetHotbarID _playerref)))
    (bind _values_2 (Utilities|Map|Values (Variables|/Game/Assets/Blueprints/Player/BP_Player.BP_Player_C|GetHotbarCount _playerref)))
    (if (> (Utilities|Array|Get(acopy) _values_2 (Utilities|Array|FindItem _values (Variables|Default|GetName))) 0)
      (Default|RemoveItem (Variables|Default|GetPlayerRef) (Variables|Default|GetName) 1)
      (Variables|Default|SetPlacing false)
      (Collision|SetCollisionEnabled (Variables|Default|GetStaticMesh) "QueryAndPhysics")
      (Variables|/Game/Assets/Blueprints/Player/BP_Player.BP_Player_C|SetBuildRotationMemory (Variables|Default|GetPlayerRef) (Variables|Default|GetManualRotation))
      (return true)
      (else
        (return false)))))

(fn CheckValidPlacement
  (bind _overlapping_ (CallFunction|OverlapTest))
  (LocalVariables|SetValid (not _overlapping_))
  (for (_array_element _array_index) (Utilities|Array|MakeArray false _overlapping_ (LocalVariables|GetValid))
    (Variables|/Script/Engine.PostProcessVolume|SetbUnbound (Utilities|Array|Get(acopy) (Utilities|Array|MakeArray (Variables|Default|GetPPV_Neutral) (Variables|Default|GetPPV_Red) (Variables|Default|GetPPV_Green)) _array_index) _array_element))
  (return (LocalVariables|GetValid)))

(fn OverlapTest
  (bind _returnvalue (Transformation|GetActorLocation))
  (bind _playerrotation (Variables|Default|GetPlayerRotation))
  (bind _manualrotation (Variables|Default|GetManualRotation))
  (bind _playerrotation_2 (Variables|Default|GetPlayerRotation))
  (bind _manualrotation_2 (Variables|Default|GetManualRotation))
  (bind _playerrotation_3 (Variables|Default|GetPlayerRotation))
  (bind _manualrotation_3 (Variables|Default|GetManualRotation))
  (bind _returnvalue_2 (Math|Rotator|CombineRotators _playerrotation _manualrotation))
  (bind _returnvalue_3 (Math|Rotator|CombineRotators _playerrotation_2 _manualrotation_2))
  (bind _returnvalue_4 (Math|Rotator|CombineRotators _playerrotation_3 _manualrotation_3))
  (bind _returnvalue_5 (+ (.yaw _returnvalue_2) 0.1))
  (bind _returnvalue_6 (+ (.yaw _returnvalue_3) 0.1))
  (bind _returnvalue_7 (Math|Trig|Sin(Degrees) _returnvalue_6))
  (bind _returnvalue_8 (Math|Trig|Cos(Degrees) _returnvalue_5))
  (bind _returnvalue_9 (Math|Float|Sign(Float) _returnvalue_8))
  (bind _returnvalue_10 (Math|Float|Sign(Float) _returnvalue_7))
  (bind _returnvalue_11 (* _returnvalue_9 -2e+02))
  (bind _returnvalue_12 (* _returnvalue_10 2e+02))
  (bind _returnvalue_13 (+ _returnvalue (Math|Vector|MakeVector _returnvalue_12 _returnvalue_11 2e+02)))
  (bind _outhit (Class|KismetSystemLibrary|BoxTraceSingleforObjects _returnvalue_13 (+ _returnvalue_13 "0.100000,0.100000,0.100000") "185.000000,185.000000,185.000000" "0, 0, 0" (Utilities|Array|MakeArray "ObjectTypeQuery8" "ObjectTypeQuery9" "ObjectTypeQuery10") false 0 "None" true "(R=1.000000,G=0.000000,B=0.000000,A=1.000000)" "(R=0.000000,G=1.000000,B=0.000000,A=1.000000)" 0.1))
  (Utilities|IsValid (.hitcomponent _outhit)
    (:Is%20Valid
      (bind _asbp_buildable (Utilities|Casting|CastToBP_Buildable (.hitactor _outhit)))
      (if (not (Math|Boolean|ORBoolean (Utilities|Enum|Equal(Enum) (Variables|BP_Buildable_C|GetName _asbp_buildable) (Variables|Default|GetName)) (Utilities|Enum|Equal(Enum) (Collision|GetCollisionObjectType (.hitcomponent _outhit)) "ECC_GameTraceChannel2") (Utilities|Enum|Equal(Enum) (Collision|GetCollisionObjectType (.hitcomponent _outhit)) "ECC_GameTraceChannel4")))
        (return false)
        (else
          (return (Utilities|Operators|EqualEqual (Math|Rotator|MakeRotator (Math|Float|%(Float) (.roll (Transformation|GetActorRotation (.hitactor _outhit))) 3.6e+02) (Math|Float|%(Float) (.pitch (Transformation|GetActorRotation (.hitactor _outhit))) 3.6e+02) (Math|Float|%(Float) (.yaw (Transformation|GetActorRotation (.hitactor _outhit))) 3.6e+02)) (Math|Rotator|MakeRotator (Math|Float|%(Float) (.roll _returnvalue_4) 3.6e+02) (Math|Float|%(Float) (.pitch _returnvalue_4) 3.6e+02) (Math|Float|%(Float) (.yaw _returnvalue_4) 3.6e+02)) 45.0)))))))