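; World generator that streams procedural terrain around the player as chunks on a procedural mesh with collision.
; Each Tick, LoadSurroundings builds missing chunks within RenderDistance of PlayerChunk as new mesh sections and clears those out of range.
; GenerateChunk emits six unshared vertices per grid cell with sequential triangle indices, taking Z from GetNodeHeight.
; Seeded random-gradient height math appears unconnected, and Perlin map and resource spawning are stubs.
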(event EventBeginPlay)

(event EventTick
  (params (DeltaSeconds :type Float%20%28single-precision%29))
  (CallFunction|LoadSurroundings))

(fn ConstructionScript)

(fn GenerateChunk
  (params (Chunk :type Vector))
  (LocalVariables|SetOriginX (* (Math|Conversions|ToFloat(Integer) (Variables|Default|GetChunkSize)) (Variables|Default|GetStep) (.x Chunk)))
  (LocalVariables|SetOriginY (* (.y Chunk) (Math|Conversions|ToFloat(Integer) (Variables|Default|GetChunkSize)) (Variables|Default|GetStep)))
  (for _index (range 0 (Variables|Default|GetChunkSize))
    (LocalVariables|SetXIndex _index)
    (for _index_2 (range 0 (Variables|Default|GetChunkSize))
      (LocalVariables|SetYIndex _index_2)
      (LocalVariables|SetPosX (+ (LocalVariables|GetOriginX) (* (Math|Conversions|ToFloat(Integer) (LocalVariables|GetXIndex)) (Variables|Default|GetStep))))
      (LocalVariables|SetPosY (+ (LocalVariables|GetOriginY) (* (Math|Conversions|ToFloat(Integer) (LocalVariables|GetYIndex)) (Variables|Default|GetStep))))
      (bind _vertices (CallFunction|MakeVerts (LocalVariables|GetXIndex) (LocalVariables|GetYIndex) (LocalVariables|GetOriginX) (LocalVariables|GetOriginY)))
      (for _array_element _vertices
        (Utilities|Array|Add (LocalVariables|GetVertices) _array_element))))
  (Utilities|Array|Add (Variables|Default|GetLoadedChunks) Chunk)
  (bind _trianglelist (CallFunction|BuildTriangles (LocalVariables|GetVertices)))
  (return _trianglelist (LocalVariables|GetVertices) (LocalVariables|GetUVs)))

(fn ClearChunk
  (params (Chunk :type Vector))
  (Utilities|Array|RemoveItem (Variables|Default|GetLoadedChunks) Chunk)
  (Class|ProceduralMeshComponent|ClearMeshSection (Variables|Default|GetWorldMesh) (.Value (Utilities|Map|Find (Variables|Default|GetChunkIDs) Chunk))))

(fn MakeVerts
  (params (XIndex :type Integer) (YIndex :type Integer) (XOrigin :type Float%20%28double-precision%29) (YOrigin :type Float%20%28double-precision%29))
  (bind _step (Variables|Default|GetStep))
  (bind _step_2 (Variables|Default|GetStep))
  (bind _step_3 (Variables|Default|GetStep))
  (bind _step_4 (Variables|Default|GetStep))
  (bind _step_5 (Variables|Default|GetStep))
  (bind _step_6 (Variables|Default|GetStep))
  (bind _step_7 (Variables|Default|GetStep))
  (bind _step_8 (Variables|Default|GetStep))
  (bind _step_9 (Variables|Default|GetStep))
  (bind _step_10 (Variables|Default|GetStep))
  (bind _step_11 (Variables|Default|GetStep))
  (bind _step_12 (Variables|Default|GetStep))
  (bind _returnvalue (Math|Conversions|ToFloat(Integer) XIndex))
  (bind _returnvalue_2 (Math|Conversions|ToFloat(Integer) YIndex))
  (bind _returnvalue_3 (Math|Conversions|ToFloat(Integer) YIndex))
  (bind _returnvalue_4 (Math|Conversions|ToFloat(Integer) XIndex))
  (bind _returnvalue_5 (Math|Conversions|ToFloat(Integer) YIndex))
  (bind _returnvalue_6 (Math|Conversions|ToFloat(Integer) XIndex))
  (bind _returnvalue_7 (+ YIndex 1))
  (bind _returnvalue_8 (+ YIndex 1))
  (bind _returnvalue_9 (+ XIndex 1))
  (bind _returnvalue_10 (+ YIndex 1))
  (bind _returnvalue_11 (+ XIndex 1))
  (bind _returnvalue_12 (+ XIndex 1))
  (bind _returnvalue_13 (Math|Conversions|ToFloat(Integer) _returnvalue_7))
  (bind _returnvalue_14 (Math|Conversions|ToFloat(Integer) _returnvalue_8))
  (bind _returnvalue_15 (Math|Conversions|ToFloat(Integer) _returnvalue_12))
  (bind _returnvalue_16 (Math|Conversions|ToFloat(Integer) _returnvalue_11))
  (bind _returnvalue_17 (Math|Conversions|ToFloat(Integer) _returnvalue_9))
  (bind _returnvalue_18 (Math|Conversions|ToFloat(Integer) _returnvalue_10))
  (bind _returnvalue_19 (* _returnvalue_2 _step_3))
  (bind _returnvalue_20 (* _returnvalue_3 _step_5))
  (bind _returnvalue_21 (* _returnvalue_4 _step_6))
  (bind _returnvalue_22 (* _returnvalue_5 _step_7))
  (bind _returnvalue_23 (* _returnvalue_6 _step_10))
  (bind _returnvalue_24 (* _returnvalue _step_12))
  (bind _returnvalue_25 (+ _returnvalue_24 XOrigin))
  (bind _returnvalue_26 (* _returnvalue_14 _step))
  (bind _returnvalue_27 (* _returnvalue_15 _step_2))
  (bind _returnvalue_28 (* _returnvalue_16 _step_4))
  (bind _returnvalue_29 (+ _returnvalue_19 YOrigin))
  (bind _returnvalue_30 (+ _returnvalue_21 XOrigin))
  (bind _returnvalue_31 (+ _returnvalue_20 YOrigin))
  (bind _returnvalue_32 (* _returnvalue_17 _step_8))
  (bind _returnvalue_33 (+ _returnvalue_22 YOrigin))
  (bind _returnvalue_34 (* _returnvalue_18 _step_9))
  (bind _returnvalue_35 (+ _returnvalue_23 XOrigin))
  (bind _returnvalue_36 (* _returnvalue_13 _step_11))
  (bind _returnvalue_37 (+ _returnvalue_36 YOrigin))
  (bind _returnvalue_38 (+ _returnvalue_27 XOrigin))
  (bind _returnvalue_39 (+ _returnvalue_26 YOrigin))
  (bind _returnvalue_40 (+ _returnvalue_28 XOrigin))
  (bind _returnvalue_41 (+ _returnvalue_32 XOrigin))
  (bind _returnvalue_42 (+ _returnvalue_34 YOrigin))
  (return (Utilities|Array|MakeArray (Math|Vector|MakeVector _returnvalue_30 _returnvalue_31 (Utilities|GetNodeHeight _returnvalue_30 _returnvalue_31)) (Math|Vector|MakeVector _returnvalue_35 _returnvalue_42 (Utilities|GetNodeHeight _returnvalue_35 _returnvalue_42)) (Math|Vector|MakeVector _returnvalue_41 _returnvalue_33 (Utilities|GetNodeHeight _returnvalue_41 _returnvalue_33)) (Math|Vector|MakeVector _returnvalue_40 _returnvalue_29 (Utilities|GetNodeHeight _returnvalue_40 _returnvalue_29)) (Math|Vector|MakeVector _returnvalue_25 _returnvalue_37 (Utilities|GetNodeHeight _returnvalue_25 _returnvalue_37)) (Math|Vector|MakeVector _returnvalue_38 _returnvalue_39 (Utilities|GetNodeHeight _returnvalue_38 _returnvalue_39)))))

(fn LoadSurroundings
  (bind _chunk (Utilities|PlayerChunk))
  (bind _output_get (LocalVariables|SetX (* (Variables|Default|GetRender%20Distance) -1)))
  (LocalVariables|SetY (- _output_get 1))
  (for _index (range 0 (* (Variables|Default|GetRender%20Distance) 2))
    (LocalVariables|SetY (+ 1 (LocalVariables|GetY)))
    (LocalVariables|SetX (* (Variables|Default|GetRender%20Distance) -1))
    (for _index_2 (range 0 (* (Variables|Default|GetRender%20Distance) 2))
      (LocalVariables|SetX (+ (LocalVariables|GetX) 1))
      (LocalVariables|SetChunkPos (Math|Vector|MakeVector (+ (Math|Conversions|ToFloat(Integer) (LocalVariables|GetX)) (.x _chunk)) (+ (Math|Conversions|ToFloat(Integer) (LocalVariables|GetY)) (.y _chunk)) 0.0))
      (Utilities|Array|Add (LocalVariables|GetNewLoaded) (LocalVariables|GetChunkPos))
      (if (not (Utilities|Array|ContainsItem (Variables|Default|GetLoadedChunks) (LocalVariables|GetChunkPos)))
        (bind (_triangles _vertexdata) (CallFunction|GenerateChunk (LocalVariables|GetChunkPos)))
        (Class|ProceduralMeshComponent|CreateMeshSectionLinearColor (Variables|Default|GetWorldMesh) (Variables|Default|GetMaxSectionIndex) _vertexdata _triangles 0 0 0 0 0 0 0 true)
        (Utilities|Map|Add (Variables|Default|GetChunkIDs) (LocalVariables|GetChunkPos) (Variables|Default|GetMaxSectionIndex))
        (Variables|Default|SetMaxSectionIndex (+ (Variables|Default|GetMaxSectionIndex) 1)))))
  (for _array_element (Variables|Default|GetLoadedChunks)
    (if (not (Utilities|Array|ContainsItem (LocalVariables|GetNewLoaded) _array_element))
      (Class|ProceduralMeshComponent|ClearMeshSection (Variables|Default|GetWorldMesh) (.Value (Utilities|Map|Find (Variables|Default|GetChunkIDs) _array_element)))
      (Utilities|Array|RemoveItem (Variables|Default|GetLoadedChunks) _array_element))))

(fn BuildTriangles
  (params (VertexList :type Array%20of%20Vectors))
  (for _index (range 0 (Utilities|Array|Length VertexList))
    (Utilities|Array|Add (LocalVariables|GetTriangles) _index))
  (return (LocalVariables|GetTriangles)))

(fn SpawnResourceNode
  (params (Biome%20ID :type Integer)))

(fn GeneratePerlinMap
  (params (GridFactor :type Float%20%28double-precision%29))
  (LocalVariables|SetGridStep (* GridFactor (Variables|Default|GetStep))))