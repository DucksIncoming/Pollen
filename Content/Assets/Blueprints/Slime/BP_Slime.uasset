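; Hopping slime enemy that chases the player and applies damage every tick they overlap its mesh.
; Range-limited line traces refresh a short aggression timer, steering it toward the player's last seen position; otherwise it wanders.
; Movement combines an upward velocity kick when grounded with direct offsets toward the target.
; SpawnSlime sets stats and color; wandering uses sine-hash pseudo-randomness from time, position and world seed.
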(event EventBeginPlay
  (bind _asbp_player (Utilities|Casting|CastToBP_Player (Game|GetPlayerCharacter 0)))
  (Variables|Default|SetPlayerRef _asbp_player)
  (bind _returnvalue (Actor|GetActorOfClass "/Game/Assets/Blueprints/World/WorldGenerator.WorldGenerator_C"))
  (bind _output_get (Variables|Default|SetWorldGenerator _returnvalue))
  (Variables|Default|SetWorld%20Mesh (Variables|/Game/Assets/Blueprints/World/WorldGenerator.WorldGenerator_C|GetWorldMesh _output_get)))

(event EventTick
  (params (DeltaSeconds :type Float%20%28single-precision%29))
  (Utilities|FlowControl|Sequence
    (:then_0
      (bind _outactors (Collision|ComponentOverlapActors (Variables|Default|GetStaticMesh) (Math|Transform|MakeTransform (Transformation|GetWorldLocation (Variables|Default|GetStaticMesh)) "0, 0, 0" "1.000000,1.000000,1.000000") (Utilities|Array|MakeArray "ObjectTypeQuery3") "/Game/Assets/Blueprints/Player/BP_Player.BP_Player_C"))
      (for _array_element _outactors
        (bind _asbp_player (Utilities|Casting|CastToBP_Player _array_element))
        (Default|DamagePlayer _asbp_player (Variables|Default|GetAttackDamage))))
    (:then_1
      (Transformation|SetWorldRotation (Variables|Default|GetStaticMesh) "0, 0, 0" false false)
      (CallFunction|CalculateAggression DeltaSeconds)
      (if (> (Variables|Default|GetAggressionTimer) 0.0)
        (CallFunction|ChasePlayer DeltaSeconds)
        (CallFunction|WalktoPoint (Variables|Default|GetWalkTarget) DeltaSeconds)
        (else
          (CallFunction|Wander DeltaSeconds)
          (CallFunction|WalktoPoint (Variables|Default|GetWalkTarget) DeltaSeconds))))))

(fn ConstructionScript)

(fn SpawnSlime
  (params (HP :type Float%20%28double-precision%29) (AttackDmg :type Float%20%28double-precision%29) (Transform :type Transform) (Color :type Linear%20Color%20Structure))
  (Transformation|SetActorTransform Transform)
  (Variables|Default|SetHP HP)
  (Variables|Default|SetPacified false)
  (Variables|Default|SetAttackDamage AttackDmg)
  (bind _returnvalue (Rendering|Material|CreateDynamicMaterialInstance (Variables|Default|GetStaticMesh) 0 "/Game/Assets/Blueprints/Slime/SlimeColors/Slime_Emissive.Slime_Emissive" "None" :!class /Script/Engine.PrimitiveComponent))
  (Rendering|Material|SetVectorParameterValue _returnvalue "Color" Color :!class /Script/Engine.MaterialInstanceDynamic))

(fn CheckPlayerVisibility
  (bind _staticmesh (Variables|Default|GetStaticMesh))
  (bind _playerref (Variables|Default|GetPlayerRef))
  (bind _returnvalue (Transformation|GetWorldLocation _staticmesh))
  (bind _camera (Variables|/Game/Assets/Blueprints/Player/BP_Player.BP_Player_C|GetCamera _playerref))
  (bind _returnvalue_2 (Transformation|GetWorldLocation _camera))
  (bind _outhit (Collision|LineTraceForObjects _returnvalue (Utilities|Array|Get(acopy) (Utilities|Array|MakeArray _returnvalue _returnvalue_2) (Math|Conversions|ToInteger(Boolean) (< (Math|Vector|Distance(Vector) _returnvalue _returnvalue_2) 1.8e+03))) (Utilities|Array|MakeArray "ObjectTypeQuery3" "ObjectTypeQuery1" "ObjectTypeQuery9" "ObjectTypeQuery8") false 0 "None"))
  (Utilities|Casting|CastToPawn (.hitactor _outhit)
    (:then
      (return true))
    (:CastFailed
      (return false))))

(fn CalculateAggression
  (params (DeltaTime :type Float%20%28double-precision%29))
  (bind _visible_ (CallFunction|CheckPlayerVisibility))
  (if _visible_
    (Variables|Default|SetAggressive true)
    (Variables|Default|SetAggressionTimer 3.0)
    (else
      (bind _output_get (Variables|Default|SetAggressionTimer (- (Variables|Default|GetAggressionTimer) DeltaTime)))
      (Variables|Default|SetAggressive (> _output_get 0.0)))))

(fn ChasePlayer
  (params (DeltaTime :type Float%20%28double-precision%29))
  (bind _visible_ (CallFunction|CheckPlayerVisibility))
  (if _visible_
    (Variables|Default|SetPlayerMemory (Transformation|GetWorldLocation (Variables|/Game/Assets/Blueprints/Player/BP_Player.BP_Player_C|GetCamera (Variables|Default|GetPlayerRef)))))
  (Variables|Default|SetWalkTarget (Variables|Default|GetPlayerMemory)))

(fn Wander
  (params (DeltaTime :type Float%20%28double-precision%29))
  (Variables|Default|SetWanderTimer (+ DeltaTime (Variables|Default|GetWanderTimer)))
  (if (> (Variables|Default|GetWanderTimer) (Variables|Default|GetWanderThreshold))
    (Variables|Default|SetWanderTimer 0.0)
    (bind _random (Utilities|SemirandomFloat 3.0 9.0)
      (:%20%20
        (Variables|Default|SetWanderThreshold _random)
        (bind _vector (Utilities|RandomVector -6e+02 6e+02)
          (:%20%20
            (Variables|Default|SetWalkTarget (+ _vector (Transformation|GetWorldLocation (Variables|Default|GetStaticMesh))))))))))

(fn WalktoPoint
  (params (Position :type Vector) (DeltaTime :type Float%20%28double-precision%29))
  (Utilities|FlowControl|Sequence
    (:then_0
      (bind _onfloor (CallFunction|IsonGround))
      (if _onfloor
        (Physics|SetPhysicsLinearVelocity (Variables|Default|GetStaticMesh) "0, 0,500.000000" false "None")))
    (:then_1
      (Transformation|AddWorldOffset (Variables|Default|GetStaticMesh) (* (Math|Vector|GetUnitDirection(Vector) (Transformation|GetWorldLocation (Variables|Default|GetStaticMesh)) Position) (Variables|Default|GetWalkSpeed) DeltaTime) false false))))

(fn IsonGround
  (bind _staticmesh (Variables|Default|GetStaticMesh))
  (bind _returnvalue (Transformation|GetWorldLocation _staticmesh))
  (bind _returnvalue_2 (Collision|LineTraceForObjects _returnvalue (- _returnvalue "0,0,20.000000") (Utilities|Array|MakeArray "ObjectTypeQuery1" "ObjectTypeQuery9" "ObjectTypeQuery8") false 0 "None" true "(R=1.000000,G=0.000000,B=0.000000,A=1.000000)" "(R=0.000000,G=1.000000,B=0.000000,A=1.000000)" 0.1))
  (return _returnvalue_2))