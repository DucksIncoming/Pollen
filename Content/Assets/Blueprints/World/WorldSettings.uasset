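; WorldSettings applies game quality and player settings, starting from a Custom preset with short render distance on BeginPlay.
; UpdatePreset expands Potato, Medium and High into preset values and passes Custom through, while Low returns an empty result, its values left unwired.
; UpdateSettings pushes the result to the WorldGenerator, GameUserSettings and player, deriving sprint FOV from base FOV and scaling quality fractions into integer levels, without calling ApplySettings.
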(event EventBeginPlay
  (bind _asbp_player (Utilities|Casting|CastToBP_Player (Game|GetPlayerCharacter 0)))
  (Variables|Default|SetPlayerRef _asbp_player)
  (bind _returnvalue (Actor|GetActorOfClass "/Game/Assets/Blueprints/World/WorldGenerator.WorldGenerator_C"))
  (Variables|Default|SetWorldGenerator _returnvalue)
  (CallFunction|UpdateSettings (Utilities|Struct|MakeGameSettings "Custom" 2 "(X=100.000000,Y=100.000000)" 0.5 0.5 1e+02 true)))

(fn ConstructionScript)

(fn UpdatePreset
  (params (Settings :type Game%20Settings%20Structure))
  (switch name (.qualitypreset Settings)
    (:Default
      (return (Utilities|Struct|MakeGameSettings "Custom" (.renderdistance Settings) (.resolution Settings) (.texturesize Settings) (.shadowquality Settings) (.fov Settings) (.itemphysics Settings))))
    (:Potato
      (return (Utilities|Struct|MakeGameSettings "Potato" 2 (.resolution Settings) 0.25 0.0 (.fov Settings))))
    (:Low
      (return ""))
    (:Medium
      (return (Utilities|Struct|MakeGameSettings "Medium" 4 (.resolution Settings) 0.75 0.75 (.fov Settings) true)))
    (:High
      (return (Utilities|Struct|MakeGameSettings "High" 5 (.resolution Settings) 1.0 1.0 (.fov Settings) true)))))

(fn UpdateSettings
  (params (Settings :type Game%20Settings%20Structure))
  (bind _playerref (Variables|Default|GetPlayerRef))
  (bind _newsettings (CallFunction|UpdatePreset Settings))
  (LocalVariables|SetCurrentSettings _newsettings)
  (Variables|/Game/Assets/Blueprints/World/WorldGenerator.WorldGenerator_C|SetRender%20Distance (Variables|Default|GetWorldGenerator) (.renderdistance (LocalVariables|GetCurrentSettings)))
  (bind _returnvalue (Settings|GetGameUserSettings))
  (Class|GameUserSettings|SetScreenResolution _returnvalue (Class|KismetMathLibrary|ToIntPoint(Vector2D) (.resolution (LocalVariables|GetCurrentSettings))))
  (Class|GameUserSettings|SetTextureQuality _returnvalue (Math|Float|Floor (* (.texturesize (LocalVariables|GetCurrentSettings)) 4.0)))
  (Class|GameUserSettings|SetShadowQuality _returnvalue (Math|Float|Floor (* (.shadowquality (LocalVariables|GetCurrentSettings)) 4.0)))
  (bind _output_get (Variables|/Game/Assets/Blueprints/Player/BP_Player.BP_Player_C|SetDefaultFOV _playerref (.fov (LocalVariables|GetCurrentSettings))))
  (Variables|/Game/Assets/Blueprints/Player/BP_Player.BP_Player_C|SetSprintFOV _playerref (+ _output_get (* (.fov (LocalVariables|GetCurrentSettings)) 0.1)))
  (Variables|/Game/Assets/Blueprints/Player/BP_Player.BP_Player_C|SetUseItemPhysics _playerref (.itemphysics (LocalVariables|GetCurrentSettings))))