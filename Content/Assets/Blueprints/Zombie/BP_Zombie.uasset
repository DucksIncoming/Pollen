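; Zombie enemy that wanders, chases the player on sight and deals timed melee damage with knockback, using direct capsule offsets for movement.
; Tick drives behavior: range-limited line traces trigger chasing with short last-seen memory, while nearby fully grown flowers suppress chasing but not attacks.
; Wandering uses a sine-hash random built from time, position and world seed.
; SpawnZombie sets stats and random clothing colors; death enables mesh physics before timed despawn.
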(event EventBeginPlay
  (bind _asbp_player (Utilities|Casting|CastToBP_Player (Game|GetPlayerCharacter 0)))
  (Variables|Default|SetPlayerRef _asbp_player)
  (bind _returnvalue (Actor|GetActorOfClass "/Game/Assets/Blueprints/World/WorldGenerator.WorldGenerator_C"))
  (Variables|Default|SetWorldGenerator _returnvalue))

(event EventTick
  (params (DeltaSeconds :type Float%20%28single-precision%29))
  (CallFunction|IsNearFlower)
  (Variables|Default|SetDeltaTime DeltaSeconds)
  (if (not (Variables|Default|GetDead))
    (CallFunction|AttemptDamagePlayer)
    (Utilities|FlowControl|Sequence
      (:then_0
        (bind _visible_ (CallFunction|CheckPlayerVisibility))
        (if (and (or _visible_ (> (Variables|Default|GetAggressionTimer) 0.0)) (not (Variables|Default|GetPacified)))
          (CallFunction|ChasePlayer)
          (else
            (CallFunction|Wander))))
      (:then_1
        (if (<= (Variables|Default|GetHP) 0.0)
          (CallFunction|Die))))
    (else
      (bind _output_get (Variables|Default|SetDespawnTimer (- (Variables|Default|GetDespawnTimer) (Variables|Default|GetDeltaTime))))
      (if (<= _output_get 0.0)
        (Actor|DestroyActor)))))

(fn ConstructionScript)

(fn CheckPlayerVisibility
  (bind _mesh (Variables|Character|GetMesh))
  (bind _playerref (Variables|Default|GetPlayerRef))
  (bind _returnvalue (Transformation|GetWorldLocation _mesh))
  (bind _camera (Variables|/Game/Assets/Blueprints/Player/BP_Player.BP_Player_C|GetCamera _playerref))
  (bind _returnvalue_2 (Transformation|GetWorldLocation _camera))
  (bind _outhit (Collision|LineTraceForObjects _returnvalue (Utilities|Array|Get(acopy) (Utilities|Array|MakeArray _returnvalue _returnvalue_2) (Math|Conversions|ToInteger(Boolean) (< (Math|Vector|Distance(Vector) _returnvalue _returnvalue_2) (Variables|Default|GetSensoryRadius)))) (Utilities|Array|MakeArray "ObjectTypeQuery9" "ObjectTypeQuery8" "ObjectTypeQuery13") false 0 "None" true "(R=1.000000,G=0.000000,B=0.000000,A=1.000000)" "(R=0.000000,G=1.000000,B=0.000000,A=1.000000)" 0.1))
  (Utilities|IsValid (.hitactor _outhit)
    (:Is%20Valid
      (Utilities|Casting|CastToBP_Player (.hitactor _outhit)
        (:then
          (return true))
        (:CastFailed
          (return false))))))

(fn SpawnZombie
  (params (HP :type Float%20%28double-precision%29) (AttackDmg :type Float%20%28double-precision%29) (Transform :type Transform))
  (Transformation|SetActorTransform Transform)
  (Variables|Default|SetHP HP)
  (Variables|Default|SetPacified false)
  (Variables|Default|SetAttackDmg AttackDmg)
  (for _index (range 0 2)
    (bind _returnvalue (Rendering|Material|CreateDynamicMaterialInstance (Variables|Character|GetMesh) (Utilities|Array|Get(acopy) (Utilities|Array|MakeArray 0 2 3) _index) (Utilities|Array|Get(acopy) (Utilities|Array|MakeArray "/Game/Assets/Models/Materials/Zombie/ZombieShirt.ZombieShirt" "/Game/Assets/Models/Materials/Zombie/ZombiePants.ZombiePants" "/Game/Assets/Models/Materials/Zombie/ZombieShoes.ZombieShoes") _index) "None" :!class /Script/Engine.PrimitiveComponent))
    (Rendering|Material|SetVectorParameterValue _returnvalue "Param" (Utilities|Array|Get(acopy) (Utilities|Array|MakeArray (Utilities|Array|Get(acopy) (LocalVariables|GetShirtColors) (Math|Random|RandomIntegerinRange 0 (- (Utilities|Array|Length (LocalVariables|GetShirtColors)) 1))) (Utilities|Array|Get(acopy) (LocalVariables|GetPantsColors) (Math|Random|RandomIntegerinRange 0 (- (Utilities|Array|Length (LocalVariables|GetPantsColors)) 1))) (Utilities|Array|Get(acopy) (LocalVariables|GetShoeColors) (Math|Random|RandomIntegerinRange 0 (- (Utilities|Array|Length (LocalVariables|GetShoeColors)) 1)))) _index) :!class /Script/Engine.MaterialInstanceDynamic)))

(fn WalktoPoint
  (params (Position :type Vector) (DeltaTime :type Float%20%28double-precision%29) (Chasing :type Boolean))
  (bind _capsulecomponent (Variables|Collision|GetCapsuleComponent))
  (bind _returnvalue (Transformation|GetWorldLocation _capsulecomponent))
  (bind _returnvalue_2 (Math|Vector|GetUnitDirection(Vector) _returnvalue Position))
  (LocalVariables|SetActiveWalkSpeed (Utilities|Array|Get(acopy) (Utilities|Array|MakeArray (Variables|Default|GetWalkSpeed) (Variables|Default|GetChaseSpeed)) (Math|Conversions|ToInteger(Boolean) Chasing)))
  (if (Utilities|Operators|NotEqual(!=) _returnvalue Position 1e+01)
    (Transformation|AddLocalOffset (Variables|Collision|GetCapsuleComponent) (* _returnvalue_2 (Variables|Default|GetDeltaTime) (Variables|Default|GetWalkSpeed)) false false)
    (Transformation|SetWorldRotation (Variables|Character|GetMesh) (Math|Rotator|MakeRotator 0.0 0.0 (Math|Float|Lerp (.yaw (Transformation|GetWorldRotation (Variables|Character|GetMesh))) (.yaw (Math|Rotator|MakeRotfromX _returnvalue_2)) (- 1.0 (Math|Float|Power 0.01 (Variables|Default|GetDeltaTime))))) false false)))

(fn Die
  (Physics|SetSimulatePhysics (Variables|Character|GetMesh) true)
  (Variables|Default|SetDead true)
  (Physics|SetSimulatePhysics (Variables|Collision|GetCapsuleComponent) false)
  (Variables|Default|SetDespawnTimer 1e+01))

(fn ChasePlayer
  (bind _playerref (Variables|Default|GetPlayerRef))
  (bind _camera (Variables|/Game/Assets/Blueprints/Player/BP_Player.BP_Player_C|GetCamera _playerref))
  (bind _returnvalue (Transformation|GetWorldLocation _camera))
  (bind _visible_ (CallFunction|CheckPlayerVisibility))
  (if _visible_
    (CallFunction|WalktoPoint _returnvalue (Variables|Default|GetDeltaTime) false)
    (Variables|Default|SetPlayerMemory _returnvalue)
    (Variables|Default|SetAggressionTimer 3.0)
    (else
      (CallFunction|WalktoPoint (Variables|Default|GetPlayerMemory) (Variables|Default|GetDeltaTime) false)
      (Variables|Default|SetAggressionTimer (- (Variables|Default|GetAggressionTimer) (Variables|Default|GetDeltaTime))))))

(fn Wander
  (if (> (Variables|Default|GetWanderTimer) (Variables|Default|GetWanderThreshold))
    (bind _output (Utilities|RandomFloat 6.0 15.0)
      (:%20%20
        (Variables|Default|SetWanderThreshold _output)
        (bind _output_2 (Utilities|RandomFloat -1.8e+02 1.8e+02)
          (:%20%20
            (bind _output_3 (Utilities|RandomFloat 1.5e+02 5e+02)
              (:%20%20
                (Variables|Default|SetWalkTarget (* (Math|Vector|RotateVector (Math|Vector|GetForwardVector (Variables|Collision|GetCapsuleComponent)) (Math|Rotator|MakeRotator 0.0 0.0 _output_2)) _output_3))
                (Variables|Default|SetWanderTimer 0.0)))))))
    (else
      (Variables|Default|SetWanderTimer (+ (Variables|Default|GetWanderTimer) (Variables|Default|GetDeltaTime)))
      (CallFunction|WalktoPoint (Variables|Default|GetWalkTarget) (Variables|Default|GetDeltaTime) false))))

(fn IsNearFlower
  (bind _capsulecomponent (Variables|Collision|GetCapsuleComponent))
  (bind _returnvalue (Transformation|GetWorldLocation _capsulecomponent))
  (Variables|Default|SetPacified false)
  (bind _outhits (Class|KismetSystemLibrary|BoxTraceMultiforObjects _returnvalue (+ _returnvalue 0.1) "800.000000,800.000000,800.000000" "0, 0, 0" (Utilities|Array|MakeArray "ObjectTypeQuery10") false 0 "None" true))
  (bind _array_element (Utilities|Array|ForEachLoopwithBreak _outhits :!label _label)
    (:LoopBody
      (bind _asbp_flower (Utilities|Casting|CastToBP_Flower (.hitactor _array_element)))
      (if (Variables|/Game/Assets/Blueprints/Building/BP_Flower.BP_Flower_C|GetFullyGrown _asbp_flower)
        (Variables|Default|SetPacified true)
        (goto _label Break)))
    (:Completed
      (return (Variables|Default|GetPacified)))))

(fn AttemptDamagePlayer
  (if (and (> (Variables|Default|GetDamageTimer) 1.0) (<= (Math|Vector|Distance(Vector) (Transformation|GetWorldLocation (Variables|Collision|GetCapsuleComponent)) (Transformation|GetWorldLocation (Variables|/Game/Assets/Blueprints/Player/BP_Player.BP_Player_C|GetCamera (Variables|Default|GetPlayerRef)))) 1.5e+02))
    (Variables|Default|SetDamageTimer 0.0)
    (Default|DamagePlayer (Variables|Default|GetPlayerRef) (Variables|Default|GetAttackDmg) (Math|Vector|GetUnitDirection(Vector) (Transformation|GetWorldLocation (Variables|Collision|GetCapsuleComponent)) (Transformation|GetWorldLocation (Variables|/Game/Assets/Blueprints/Player/BP_Player.BP_Player_C|GetCamera (Variables|Default|GetPlayerRef)))))
    (else
      (Variables|Default|SetDamageTimer (+ (Variables|Default|GetDamageTimer) (Variables|Default|GetDeltaTime))))))